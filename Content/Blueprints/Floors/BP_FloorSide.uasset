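; BP_FloorSide is a floor-side Blueprint that procedurally scatters randomly scaled mesh instances inside a box volume.
; After the parent construction script runs, it moves the InstancedStaticMesh to the Box's relative location, used as a world position, and clears old instances.
; It then adds a fixed batch at random points in the Box bounds, with X and Y scales from MinXY–MaxXY and a separately randomized Z scale.
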(fn ConstructionScript
  (bind _box (Variables|Default|GetBox))
  (bind (_origin _boxextent) (Collision|GetComponentBounds _box))
  (|CallParentFunction)
  (Transformation|SetWorldLocation (Variables|Default|GetInstancedStaticMesh) (Variables|/Script/Engine.SceneComponent|GetRelativeLocation (Variables|Default|GetBox)) false false)
  (Components|InstancedStaticMesh|ClearInstances (Variables|Default|GetInstancedStaticMesh))
  (for _index (range 0 10)
    (Components|InstancedStaticMesh|AddInstance (Variables|Default|GetInstancedStaticMesh) (Math|Transform|MakeTransform (Math|Random|RandomPointinBoundingBox _origin _boxextent) "0, 0, 0" (Math|Vector|MakeVector (Math|Random|RandomFloatinRange (Variables|Default|GetMinXY) (Variables|Default|GetMaxXY)) (Math|Random|RandomFloatinRange (Variables|Default|GetMinXY) (Variables|Default|GetMaxXY)) (Math|Random|RandomFloatinRange 2.0 2e+01))))))