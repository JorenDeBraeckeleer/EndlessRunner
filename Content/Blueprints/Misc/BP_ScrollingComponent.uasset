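; BP_ScrollingComponent is a component that scrolls its owning actor in step with the level's speed.
; On BeginPlay it caches the level manager, printing a message if none exists.
; While the manager is playing, Tick scales the owner's forward vector by LevelSpeed, delta time and MoveMultiplier.
; It applies the result as a non-swept local offset, although that forward vector is in world space.
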(event EventBeginPlay
  (bind (_output _isvalid) (CallFunction|GetLevelManager))
  (if _isvalid
    (Variables|Default|SetLevelManagerRef _output)
    (else
      (Development|PrintString "No levelmanager found. Every level needs a manager."))))

(event EventTick
  (params (DeltaSeconds :type Float%20%28single-precision%29))
  (bind _levelmanagerref (Variables|Default|GetLevelManagerRef))
  (Variables|Default|SetDeltaSeconds DeltaSeconds)
  (Utilities|IsValid _levelmanagerref
    (:Is%20Valid
      (if (Variables|/Game/Blueprints/Game/BP_LevelManager.BP_LevelManager_C|GetIsPlaying _levelmanagerref)
        (bind _output_get (Variables|Default|SetMovement (* (* (Transformation|GetActorForwardVector (Components|GetOwner)) (Variables|/Game/Blueprints/Game/BP_LevelManager.BP_LevelManager_C|GetLevelSpeed (Variables|Default|GetLevelManagerRef))) (Variables|Default|GetDeltaSeconds))))
        (bind _output_get_2 (Variables|Default|SetMovement (* _output_get (Variables|Default|GetMoveMultiplier))))
        (Transformation|AddActorLocalOffset (Components|GetOwner) _output_get_2 false false)))))