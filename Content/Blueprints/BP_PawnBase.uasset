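; Base player pawn for a lane-based runner that hops between lanes, shoots, and dies on obstacle hits with an explosion and end-camera blend.
; Timeline lerps move it one lane, and a short double-tap window queues a second move.
; Tick handles that window and cooldown-limited held fire using the level manager's bullet count.
; Power-up functions provide timed speed boost and score multiplier through the level manager, plus an obstacle-clearing bomb.
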(event EventBeginPlay
  (CallFunction|Initialize))

(event EventTick
  (params (DeltaSeconds :type Float%20%28single-precision%29))
  (Utilities|FlowControl|Sequence
    (:then_0
      (if (Variables|Default|GetCanDoubleTapLeft)
        (Variables|Default|SetTimerDoubleTapLeft (- (Variables|Default|GetTimerDoubleTapLeft) DeltaSeconds))
        (if (<= (Variables|Default|GetTimerDoubleTapLeft) 0.0)
          (Variables|Default|SetCanDoubleTapLeft false))
        (else
          (Variables|Default|SetTimerDoubleTapLeft 0.25))))
    (:then_1
      (if (Variables|Default|GetCanDoubleTapRight)
        (Variables|Default|SetTimerDoubleTapRight (- (Variables|Default|GetTimerDoubleTapRight) DeltaSeconds))
        (if (<= (Variables|Default|GetTimerDoubleTapRight) 0.0)
          (Variables|Default|SetCanDoubleTapRight false))
        (else
          (Variables|Default|SetTimerDoubleTapRight 0.25))))
    (:then_2
      (if (Variables|Default|GetHasShot)
        (bind _output_get (Variables|Default|SetShotCooldownTimer (- (Variables|Default|GetShotCooldownTimer) DeltaSeconds)))
        (if (<= _output_get 0.0)
          (Variables|Default|SetHasShot false)
          (if (Variables|Default|GetIsShooting)
            (CallFunction|ShootBullet)))
        (elif (Variables|Default|GetIsShooting)
          (CallFunction|ShootBullet))))))

(event Input|ActionEvents|InputActionMoveRight
  (params (Key :type Key%20Structure :default "None"))
  (bind _returnvalue (Transformation|GetActorLocation))
  (bind _returnvalue_2 (Transformation|GetActorLocation))
  (:Pressed
    (if (Variables|/Game/Blueprints/Game/BP_LevelManager.BP_LevelManager_C|GetIsPlaying (Variables|Default|GetLevelManagerRef)) :!label _label
      ;[1 1 1] Pressed right whilst in the right most lane
      (if (not (== (Variables|Default|GetCurrentLane) (Variables|/Game/Blueprints/Game/BP_LevelManager.BP_LevelManager_C|GetNrLanes (Variables|Default|GetLevelManagerRef))))
        (if (Variables|Default|GetIsMoving)
          (if (Variables|Default|GetCanDoubleTapRight)
            (Variables|Default|SetHasDoubleTappedRight true)
            (Variables|Default|SetCanDoubleTapRight false)
            (elif (Variables|Default|GetCanDoubleTapLeft)
              (Variables|Default|SetHasDoubleTappedRight true)
              (Variables|Default|SetCanDoubleTapLeft false)))
          (else
            (Variables|Default|SetIsMoving true)
            (Audio|PlaySoundatLocation "/Game/Assests/Sounds/Movement_Cue.Movement_Cue" (Transformation|GetActorLocation) "0, 0, 0" 1.0 1.0 0.0 0 0 0)
            (Variables|Default|SetCanDoubleTapRight true)
            (Variables|Default|SetTargetPosition (+ (.y (Transformation|GetActorLocation)) (Variables|Default|GetLaneWidth)))
            (bind _move (Timeline|MoveRight PlayFromStart)
              (:Update
                (Transformation|SetActorLocation (Math|Vector|MakeVector (.x _returnvalue_2) (Math|Float|Lerp (.y _returnvalue_2) (Variables|Default|GetTargetPosition) _move) (.z _returnvalue_2)) false false))
              (:Finished
                (Variables|Default|SetIsMoving false)
                (Math|Integer|IncrementInt (Variables|Default|GetCurrentLane)
                  (:%20%20
                    (if (Variables|Default|GetHasDoubleTappedRight)
                      (Variables|Default|SetHasDoubleTappedRight false)
                      (goto _label)
                      (elif (Variables|Default|GetHasDoubleTappedLeft)
                        (Variables|Default|SetHasDoubleTappedLeft false)
                        (if (Variables|/Game/Blueprints/Game/BP_LevelManager.BP_LevelManager_C|GetIsPlaying (Variables|Default|GetLevelManagerRef)) :!label _label_2
                          ;[1 1 1] Pressed left whilst in the left most lane
                          (if (not (<= (Variables|Default|GetCurrentLane) 1))
                            (if (Variables|Default|GetIsMoving)
                              (if (Variables|Default|GetCanDoubleTapLeft)
                                (Variables|Default|SetHasDoubleTappedLeft true)
                                (Variables|Default|SetCanDoubleTapLeft false)
                                (elif (Variables|Default|GetCanDoubleTapRight)
                                  (Variables|Default|SetHasDoubleTappedLeft true)
                                  (Variables|Default|SetCanDoubleTapRight false)))
                              (else
                                (Variables|Default|SetIsMoving true)
                                (Audio|PlaySoundatLocation "/Game/Assests/Sounds/Movement_Cue.Movement_Cue" (Transformation|GetActorLocation) "0, 0, 0" 1.0 1.0 0.0 0 0 0)
                                (Variables|Default|SetCanDoubleTapLeft true)
                                (Variables|Default|SetTargetPosition (- (.y (Transformation|GetActorLocation)) (Variables|Default|GetLaneWidth)))
                                (bind _move_2 (Timeline|MoveLeft PlayFromStart)
                                  (:Update
                                    (Transformation|SetActorLocation (Math|Vector|MakeVector (.x _returnvalue) (Math|Float|Lerp (.y _returnvalue) (Variables|Default|GetTargetPosition) _move_2) (.z _returnvalue)) false false))
                                  (:Finished
                                    (Variables|Default|SetIsMoving false)
                                    (Math|Integer|DecrementInt (Variables|Default|GetCurrentLane)
                                      (:%20%20
                                        (if (Variables|Default|GetHasDoubleTappedLeft)
                                          (Variables|Default|SetHasDoubleTappedLeft false)
                                          (goto _label_2)
                                          (elif (Variables|Default|GetHasDoubleTappedRight)
                                            (Variables|Default|SetHasDoubleTappedRight false)
                                            (goto _label)))))))))))))))))))))))

(event Input|ActionEvents|InputActionMoveLeft
  (params (Key :type Key%20Structure :default "None"))
  (bind _returnvalue (Transformation|GetActorLocation))
  (bind _returnvalue_2 (Transformation|GetActorLocation))
  (:Pressed
    (if (Variables|/Game/Blueprints/Game/BP_LevelManager.BP_LevelManager_C|GetIsPlaying (Variables|Default|GetLevelManagerRef)) :!label _label
      ;[1 1 1] Pressed left whilst in the left most lane
      (if (not (<= (Variables|Default|GetCurrentLane) 1))
        (if (Variables|Default|GetIsMoving)
          (if (Variables|Default|GetCanDoubleTapLeft)
            (Variables|Default|SetHasDoubleTappedLeft true)
            (Variables|Default|SetCanDoubleTapLeft false)
            (elif (Variables|Default|GetCanDoubleTapRight)
              (Variables|Default|SetHasDoubleTappedLeft true)
              (Variables|Default|SetCanDoubleTapRight false)))
          (else
            (Variables|Default|SetIsMoving true)
            (Audio|PlaySoundatLocation "/Game/Assests/Sounds/Movement_Cue.Movement_Cue" (Transformation|GetActorLocation) "0, 0, 0" 1.0 1.0 0.0 0 0 0)
            (Variables|Default|SetCanDoubleTapLeft true)
            (Variables|Default|SetTargetPosition (- (.y (Transformation|GetActorLocation)) (Variables|Default|GetLaneWidth)))
            (bind _move (Timeline|MoveLeft PlayFromStart)
              (:Update
                (Transformation|SetActorLocation (Math|Vector|MakeVector (.x _returnvalue) (Math|Float|Lerp (.y _returnvalue) (Variables|Default|GetTargetPosition) _move) (.z _returnvalue)) false false))
              (:Finished
                (Variables|Default|SetIsMoving false)
                (Math|Integer|DecrementInt (Variables|Default|GetCurrentLane)
                  (:%20%20
                    (if (Variables|Default|GetHasDoubleTappedLeft)
                      (Variables|Default|SetHasDoubleTappedLeft false)
                      (goto _label)
                      (elif (Variables|Default|GetHasDoubleTappedRight)
                        (Variables|Default|SetHasDoubleTappedRight false)
                        (if (Variables|/Game/Blueprints/Game/BP_LevelManager.BP_LevelManager_C|GetIsPlaying (Variables|Default|GetLevelManagerRef)) :!label _label_2
                          ;[1 1 1] Pressed right whilst in the right most lane
                          (if (not (== (Variables|Default|GetCurrentLane) (Variables|/Game/Blueprints/Game/BP_LevelManager.BP_LevelManager_C|GetNrLanes (Variables|Default|GetLevelManagerRef))))
                            (if (Variables|Default|GetIsMoving)
                              (if (Variables|Default|GetCanDoubleTapRight)
                                (Variables|Default|SetHasDoubleTappedRight true)
                                (Variables|Default|SetCanDoubleTapRight false)
                                (elif (Variables|Default|GetCanDoubleTapLeft)
                                  (Variables|Default|SetHasDoubleTappedRight true)
                                  (Variables|Default|SetCanDoubleTapLeft false)))
                              (else
                                (Variables|Default|SetIsMoving true)
                                (Audio|PlaySoundatLocation "/Game/Assests/Sounds/Movement_Cue.Movement_Cue" (Transformation|GetActorLocation) "0, 0, 0" 1.0 1.0 0.0 0 0 0)
                                (Variables|Default|SetCanDoubleTapRight true)
                                (Variables|Default|SetTargetPosition (+ (.y (Transformation|GetActorLocation)) (Variables|Default|GetLaneWidth)))
                                (bind _move_2 (Timeline|MoveRight PlayFromStart)
                                  (:Update
                                    (Transformation|SetActorLocation (Math|Vector|MakeVector (.x _returnvalue_2) (Math|Float|Lerp (.y _returnvalue_2) (Variables|Default|GetTargetPosition) _move_2) (.z _returnvalue_2)) false false))
                                  (:Finished
                                    (Variables|Default|SetIsMoving false)
                                    (Math|Integer|IncrementInt (Variables|Default|GetCurrentLane)
                                      (:%20%20
                                        (if (Variables|Default|GetHasDoubleTappedRight)
                                          (Variables|Default|SetHasDoubleTappedRight false)
                                          (goto _label_2)
                                          (elif (Variables|Default|GetHasDoubleTappedLeft)
                                            (Variables|Default|SetHasDoubleTappedLeft false)
                                            (goto _label)))))))))))))))))))))))

(event Input|ActionEvents|InputActionShoot
  (params (Key :type Key%20Structure :default "None"))
  (:Pressed
    (CallFunction|ShootBullet)
    (Variables|Default|SetIsShooting true))
  (:Released
    (Variables|Default|SetIsShooting false)))

(event Input|ActionEvents|InputActionUse
  (params (Key :type Key%20Structure :default "None")))

(fn ConstructionScript)

(fn Initialize
  (bind (_output _isvalid) (CallFunction|GetLevelManager))
  (if _isvalid
    (Variables|Default|SetLevelManagerRef _output)
    (Variables|Default|SetCurrentLane (+ (/ (Variables|/Game/Blueprints/Game/BP_LevelManager.BP_LevelManager_C|GetNrLanes (Variables|Default|GetLevelManagerRef)) 2) 1))
    (Variables|Default|SetLaneWidth (Variables|/Game/Blueprints/Game/BP_LevelManager.BP_LevelManager_C|GetLaneWidth (Variables|Default|GetLevelManagerRef)))
    (bind _outactors (Actor|GetAllActorswithTag "EndCamera"))
    (Variables|Default|SetEndCameraRef (Utilities|Array|Get(acopy) _outactors))
    (Class|PlayerController|SetAudioListenerOverride (Game|GetPlayerController 0) (Variables|Default|GetCharListenerPos) "0, 0, 0" "0, 0, 0")
    (else
      (Development|PrintString "No levelmanager found. Every level needs a manager."))))

(fn HitObstacle
  (Audio|PlaySoundatLocation "/Game/Assests/Sounds/Death_Cue.Death_Cue" (Transformation|GetActorLocation) "0, 0, 0" 1.0 1.0 0.0 0 0 0)
  (Utilities|IsValid (Variables|Default|GetParticleSystem)
    (:Is%20Valid
      (Components|DestroyComponent (Variables|Default|GetParticleSystem)))
    (:Is%20Not%20Valid
      _))
  (Effects|SpawnEmitteratLocation "/Game/ExampleContent/Input_Examples/Effects/P_Pixel_Explosion_Player.P_Pixel_Explosion_Player" (Transformation|GetActorLocation) "0, 0, 0" "2.000000,2.000000,2.000000")
  (Game|Player|SetViewTargetwithBlend (Game|GetPlayerController 0) (Variables|Default|GetEndCameraRef) 2.0 "VTBlend_Linear" 0.0 false)
  (Rendering|ToggleVisibility (Variables|Default|GetPlayer) false)
  (Components|Activation|Deactivate (Variables|Default|GetAudio)))

(fn GameStarted
  (Effects|Components|ParticleSystem|SetTemplate (Variables|Default|GetParticleSystem) "/Game/ExampleContent/Input_Examples/Effects/P_Pixel_Engine.P_Pixel_Engine")
  (Components|Activation|Activate (Variables|Default|GetAudio) false))

(fn BoostStart
  (bind _levelmanagerref (Variables|Default|GetLevelManagerRef))
  (Variables|Default|SetIsBoosting true)
  (Utilities|Time|SetTimerbyFunctionName 0 "BoostEnd" 5.0)
  (bind _output_get (Variables|Default|SetOldLevelSpeeldForBoost (Variables|/Game/Blueprints/Game/BP_LevelManager.BP_LevelManager_C|GetLevelSpeed _levelmanagerref)))
  (Variables|/Game/Blueprints/Game/BP_LevelManager.BP_LevelManager_C|SetLevelSpeed _levelmanagerref (* _output_get 2.0))
  (Components|Activation|Activate (Variables|Default|GetNS_SpeedLines) false))

(fn BoostEnd
  (Variables|Default|SetIsBoosting false)
  (Variables|/Game/Blueprints/Game/BP_LevelManager.BP_LevelManager_C|SetLevelSpeed (Variables|Default|GetLevelManagerRef) (Variables|Default|GetOldLevelSpeeldForBoost))
  (Components|Activation|Deactivate (Variables|Default|GetNS_SpeedLines)))

(fn ShootBullet
  (if (not (Variables|Default|GetHasShot))
    (if (Default|HasBullets (Variables|Default|GetLevelManagerRef))
      (Game|SpawnActorfromClass "/Game/Blueprints/BP_Bullet.BP_Bullet_C" (Transformation|GetActorTransform) "Undefined" 0 1e+01 0)
      (Default|LoseBullets (Variables|Default|GetLevelManagerRef) 1)
      (Variables|Default|SetHasShot true)
      (Variables|Default|SetShotCooldownTimer (Variables|Default|GetShotCooldown)))))

(fn Boost
  (if (not (Variables|Default|GetIsBoosting))
    (CallFunction|BoostStart)))

(fn Bomb
  (bind _outactors (Actor|GetAllActorsOfClass "/Game/Blueprints/Obstacles/BP_Obstacle.BP_Obstacle_C"))
  (for _array_element _outactors
    (Default|Death _array_element)))

(fn SetScoreMultiplier
  (params (ScoreMultiplier :type Integer))
  (if (not (Variables|Default|GetHasScoreMultiplier))
    (Variables|/Game/Blueprints/Game/BP_LevelManager.BP_LevelManager_C|SetScoreMultiplier (Variables|Default|GetLevelManagerRef) ScoreMultiplier)
    (Utilities|Time|SetTimerbyFunctionName 0 "ResetScoreMultiplier" 5.0)
    (Variables|Default|SetHasScoreMultiplier true)
    (Default|ShowMultiplier (Variables|/Game/Blueprints/Game/BP_LevelManager.BP_LevelManager_C|GetHUD (Variables|Default|GetLevelManagerRef)) true)))

(fn ResetScoreMultiplier
  (Variables|/Game/Blueprints/Game/BP_LevelManager.BP_LevelManager_C|SetScoreMultiplier (Variables|Default|GetLevelManagerRef) 1)
  (Variables|Default|SetHasScoreMultiplier false)
  (Default|ShowMultiplier (Variables|/Game/Blueprints/Game/BP_LevelManager.BP_LevelManager_C|GetHUD (Variables|Default|GetLevelManagerRef)) false))