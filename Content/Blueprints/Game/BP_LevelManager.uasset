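; Level manager actor that runs the game flow from start menu through HUD play to game over, skipping the menu on restarts flagged in the game instance.
; Looping timers step LevelSpeed down and refill bullets up to a cap once play starts.
; A configurable out-of-bounds box notifies the parent of overlapping actors through GetActorHitBounds and awards score.
; Score and bullet changes are pushed to the HUD.
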(event OnComponentBeginOverlap(LevelBounds)
  (params (OverlappedComponent :type Primitive%20Component%20Object%20Reference) (OtherActor :type Actor%20Object%20Reference) (OtherComp :type Primitive%20Component%20Object%20Reference) (OtherBodyIndex :type Integer) (bFromSweep :type Boolean) (SweepResult :type Hit%20Result%20Structure%20%28by%20ref%29))
  (bind _parent (Class|BPISpawnable|GetParent(Message) OtherActor))
  (Utilities|IsValid _parent
    (:Is%20Valid
      (Default|GetActorHitBounds _parent OtherActor)
      (CallFunction|AddScore 1)
      (CallFunction|UpdateScore))))

(event Custom|UpdateBulletCount
  (if (not (>= (Variables|Default|GetBulletCount) (Variables|Default|GetMaxBulletCount)))
    (CallFunction|AddBullets 1)))

(event Custom|IncreaseSpeed
  (Variables|Default|SetLevelSpeed (- (Variables|Default|GetLevelSpeed) 25.0)))

(event Custom|StartGameEvents
  (Utilities|Time|SetTimerbyEvent (delegate Custom|IncreaseSpeed) 5.0 true)
  (Utilities|Time|SetTimerbyEvent (delegate Custom|UpdateBulletCount) 1.5 true))

(event EventBeginPlay
  (bind _returnvalue (Game|GetPlayerController 0))
  (Variables|Default|SetLevelSpeedBase (Variables|Default|GetLevelSpeed))
  (bind _asbp_pawn_base (Utilities|Casting|CastToBP_PawnBase (Game|Player|GetPlayerPawn 0)))
  (Variables|Default|SetPlayerRef _asbp_pawn_base)
  (bind _asbp_game_instance_base (Utilities|Casting|CastToBP_GameInstanceBase (Game|GetGameInstance)))
  (if (Variables|/Game/Blueprints/Game/BP_GameInstanceBase.BP_GameInstanceBase_C|GetIsRestart _asbp_game_instance_base)
    (Variables|/Game/Blueprints/Game/BP_GameInstanceBase.BP_GameInstanceBase_C|SetIsRestart _asbp_game_instance_base false)
    (CallFunction|GameStart)
    (else
      (bind _returnvalue_2 (UserInterface|CreateWidget "/Game/Blueprints/UI/BPW_StartMenu.BPW_StartMenu_C" 0 self))
      (UserInterface|Viewport|AddtoViewport _returnvalue_2 0)
      (Input|SetInputModeUIOnly _returnvalue 0 "DoNotLock")
      (Variables|/Script/Engine.PlayerController|SetbShowMouseCursor _returnvalue true))))

(fn ConstructionScript
  (Components|Box|SetBoxExtent (Variables|Default|GetLevelBounds) (Variables|Default|GetOutOfBoundBoxScale) true)
  (Transformation|SetWorldLocation (Variables|Default|GetLevelBounds) (Variables|Default|GetOutOfBoundBoxLocation) false false))

(fn GetParent
  (return 0))

(fn SetParent
  (params (Parent :type BP%20Spawner%20Base%20Object%20Reference))
  (return false))

(fn GameOver
  (bind _returnvalue (Game|GetPlayerController 0))
  (Variables|Default|SetLevelSpeed 0.0)
  (Variables|Default|SetIsPlaying false)
  (bind _returnvalue_2 (UserInterface|CreateWidget "/Game/Blueprints/UI/BPW_GameOver.BPW_GameOver_C" 0 self))
  (UserInterface|Viewport|AddtoViewport _returnvalue_2 0)
  (Input|SetInputModeUIOnly _returnvalue 0 "DoNotLock")
  (Variables|/Script/Engine.PlayerController|SetbShowMouseCursor _returnvalue true))

(fn GameStart
  (bind _returnvalue (Game|GetPlayerController 0))
  (Variables|Default|SetIsPlaying true)
  (Input|SetInputModeGameOnly _returnvalue)
  (Variables|/Script/Engine.PlayerController|SetbShowMouseCursor _returnvalue false)
  (bind _returnvalue_2 (UserInterface|CreateWidget "/Game/Blueprints/UI/BPW_HUD.BPW_HUD_C"))
  (bind _output_get (Variables|Default|SetHUD _returnvalue_2))
  (UserInterface|Viewport|AddtoViewport _output_get 0)
  (CallFunction|StartGameEvents)
  (Default|GameStarted (Variables|Default|GetPlayerRef)))

(fn UpdateScore
  (Default|SetScore (Variables|Default|GetHUD) (Variables|Default|GetScore)))

(fn AddScore
  (params (Score :type Integer))
  (Variables|Default|SetScore (+ (Variables|Default|GetScore) (* Score (Variables|Default|GetScoreMultiplier)))))

(fn AddBullets
  (params (NrBullets :type Integer))
  (bind _output_get (Variables|Default|SetBulletCount (+ (Variables|Default|GetBulletCount) NrBullets)))
  (if (>= _output_get (Variables|Default|GetMaxBulletCount))
    (Variables|Default|SetBulletCount (Variables|Default|GetMaxBulletCount)))
  (CallFunction|UpdateBullets))

(fn HasBullets
  (return (> (Variables|Default|GetBulletCount) 0)))

(fn LoseBullets
  (params (NrBullets :type Integer))
  (CallFunction|AddBullets (* NrBullets -1)))

(fn UpdateBullets
  (if (Variables|Default|GetIsPlaying)
    (Default|SetBullets (Variables|Default|GetHUD) (Variables|Default|GetBulletCount))))