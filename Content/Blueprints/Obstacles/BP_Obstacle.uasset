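; Obstacle actor that ends the game when a player pawn overlaps it and can be destroyed for score.
; Construction randomizes mesh rotation; on BeginPlay a timeline grows the mesh to a random scale, provided a level manager exists.
; Hit passes damage to the health component, whose result triggers Death: sound, explosion, actor destruction and a score update through the level manager.
; It also stores a parent reference with a getter and setter.
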(event OnComponentBeginOverlap(StaticMesh)
  (params (OverlappedComponent :type Primitive%20Component%20Object%20Reference) (OtherActor :type Actor%20Object%20Reference) (OtherComp :type Primitive%20Component%20Object%20Reference) (OtherBodyIndex :type Integer) (bFromSweep :type Boolean) (SweepResult :type Hit%20Result%20Structure%20%28by%20ref%29))
  (bind (_output _isvalid) (CallFunction|GetLevelManager))
  (bind _asbp_pawn_base (Utilities|Casting|CastToBP_PawnBase OtherActor))
  (Default|HitObstacle _asbp_pawn_base)
  (if _isvalid
    (Default|GameOver _output)
    (else
      (Development|PrintString "No levelmanager found. Every level needs a manager."))))

(event EventBeginPlay
  (bind (_output _isvalid) (CallFunction|GetLevelManager))
  (if _isvalid
    (Variables|Default|SetLevelManagerRef _output)
    (Variables|Default|SetScale (Math|Random|RandomFloatinRange 5e+01 8e+01))
    (bind _growth (Timeline|Growing PlayFromStart)
      (:Update
        (Transformation|SetWorldScale3D (Variables|Default|GetStaticMesh) (Math|Vector|MakeVector (* _growth (Variables|Default|GetScale)) (* _growth (Variables|Default|GetScale)) (* _growth (Variables|Default|GetScale)))))
      (:Finished
        (Transformation|SetWorldScale3D (Variables|Default|GetStaticMesh) (Math|Vector|MakeVector (Variables|Default|GetScale) (Variables|Default|GetScale) (Variables|Default|GetScale)))))
    (else
      (Development|PrintString "No levelmanager found. Every level needs a manager."))))

(fn ConstructionScript
  (Transformation|SetWorldRotation (Variables|Default|GetStaticMesh) (Math|Rotator|MakeRotator (Math|Random|RandomFloatinRange 0.0 3.6e+02) (Math|Random|RandomFloatinRange 0.0 3.6e+02) (Math|Random|RandomFloatinRange 0.0 3.6e+02)) false false))

(fn Death
  (bind _levelmanagerref (Variables|Default|GetLevelManagerRef))
  (Audio|PlaySoundatLocation "/Game/Assests/Sounds/Death_Cue.Death_Cue" (Transformation|GetActorLocation) "0, 0, 0" 1.0 1.0 0.0 0 0 0)
  (Effects|SpawnEmitteratLocation "/Game/ExampleContent/Input_Examples/Effects/P_Pixel_Explosion_Enemy.P_Pixel_Explosion_Enemy" (Transformation|GetActorLocation) "0, 0, 0" "5.000000,5.000000,5.000000")
  (Actor|DestroyActor)
  (Default|AddScore _levelmanagerref 2)
  (Default|UpdateScore _levelmanagerref))

(fn Hit
  (params (Damage :type Float%20%28single-precision%29))
  (Audio|SpawnSoundatLocation "/Game/Assests/Sounds/Hit_Cue.Hit_Cue" (Transformation|GetActorLocation) "0, 0, 0" 1.0 1.0 0.0 0 0)
  (bind _isdead (Default|DealDamage (Variables|Default|GetBP_HealthComponent) Damage))
  (if _isdead
    (CallFunction|Death)))

(fn GetParent
  (return (Variables|Default|GetParentRef)))

(fn SetParent
  (params (Parent :type BP%20Spawner%20Base%20Object%20Reference))
  (Variables|Default|SetParentRef Parent)
  (return false))