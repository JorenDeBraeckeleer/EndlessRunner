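; BP_Bullet is a projectile actor that damages BP_Obstacle actors it overlaps and expires after a limited lifetime.
; On spawn it plays a shot sound, caches its average mesh scale and sets a lifetime timer that shortens as level speed rises above base.
; On timeout, a Shrinking timeline scales the mesh down before destroying the actor.
; An obstacle overlap triggers a pixel explosion, destroys the bullet and passes Damage to the obstacle's Hit.
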(event OnComponentBeginOverlap(StaticMesh)
  (params (OverlappedComponent :type Primitive%20Component%20Object%20Reference) (OtherActor :type Actor%20Object%20Reference) (OtherComp :type Primitive%20Component%20Object%20Reference) (OtherBodyIndex :type Integer) (bFromSweep :type Boolean) (SweepResult :type Hit%20Result%20Structure%20%28by%20ref%29))
  (bind _asbp_obstacle (Utilities|Casting|CastToBP_Obstacle OtherActor))
  (CallFunction|Death)
  (Default|Hit _asbp_obstacle (Variables|Default|GetDamage)))

(event Custom|LifeTime
  (bind _shrink (Timeline|Shrinking PlayFromStart)
    (:Update
      (Transformation|SetWorldScale3D (Variables|Default|GetStaticMesh) (Math|Vector|MakeVector (* _shrink (Variables|Default|GetScale)) (* _shrink (Variables|Default|GetScale)) (* _shrink (Variables|Default|GetScale)))))
    (:Finished
      (Transformation|SetWorldScale3D (Variables|Default|GetStaticMesh) (Math|Vector|MakeVector 0.0 0.0 0.0))
      (Actor|DestroyActor))))

(event EventBeginPlay
  (bind (_output _isvalid) (CallFunction|GetLevelManager))
  (bind _staticmesh (Variables|Default|GetStaticMesh))
  (bind _returnvalue (Transformation|GetWorldScale _staticmesh))
  (Audio|PlaySoundatLocation "/Game/Assests/Sounds/Shot_Cue.Shot_Cue" (Transformation|GetActorLocation) "0, 0, 0" 1.0 1.0 0.0 0 0 0)
  (if _isvalid
    (Utilities|Time|SetTimerbyEvent (delegate Custom|LifeTime) (/ (Variables|Default|GetLifeTimeBase) (/ (Variables|/Game/Blueprints/Game/BP_LevelManager.BP_LevelManager_C|GetLevelSpeed _output) (Variables|/Game/Blueprints/Game/BP_LevelManager.BP_LevelManager_C|GetLevelSpeedBase _output))))
    (Variables|Default|SetScale (/ (+ (+ (.x _returnvalue) (.y _returnvalue)) (.z _returnvalue)) 3.0))))

(fn ConstructionScript)

(fn Death
  (Effects|SpawnEmitteratLocation "/Game/ExampleContent/Input_Examples/Effects/P_Pixel_Explosion.P_Pixel_Explosion" (Transformation|GetActorLocation) "0, 0, 0" "4.000000,4.000000,4.000000")
  (Actor|DestroyActor))