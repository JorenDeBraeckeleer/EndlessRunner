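; BP_SpawnerObstacle spawns obstacles at its own location, at random intervals while the level is playing.
; On BeginPlay it gets the level manager, polling each second until play starts if needed.
; A self-recalling delay loop places each obstacle through the parent's SpawnActor and stops rescheduling once play ends.
; Actors passed to GetActorHitBounds as out of bounds are destroyed.
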(event Custom|LineUpNextObstacleSpawn
  (Utilities|FlowControl|Delay (Math|Random|RandomFloatinRange (Variables|Default|GetMinDelay) (Variables|Default|GetMaxDelay)))
  (CallFunction|PlaceObstacle)
  (if (Variables|/Game/Blueprints/Game/BP_LevelManager.BP_LevelManager_C|GetIsPlaying (Variables|Default|GetLevelManagerRef))
    (CallFunction|LineUpNextObstacleSpawn)))

(event Custom|CheckIfPlaying
  (if (Variables|/Game/Blueprints/Game/BP_LevelManager.BP_LevelManager_C|GetIsPlaying (Variables|Default|GetLevelManagerRef))
    (CallFunction|LineUpNextObstacleSpawn)
    (Utilities|Time|ClearTimerbyFunctionName 0 "CheckIfPlaying")))

(event EventBeginPlay
  (bind (_output _isvalid) (CallFunction|GetLevelManager))
  (if _isvalid
    (Variables|Default|SetLevelManagerRef _output)
    (if (Variables|/Game/Blueprints/Game/BP_LevelManager.BP_LevelManager_C|GetIsPlaying (Variables|Default|GetLevelManagerRef))
      (CallFunction|LineUpNextObstacleSpawn)
      (else
        (Utilities|Time|SetTimerbyEvent (delegate Custom|CheckIfPlaying) 1.0 true)))))

(event EventGetActorHitBounds
  (params (OutOfBoundsActor :type Actor%20Object%20Reference))
  (Actor|DestroyActor OutOfBoundsActor))

(fn ConstructionScript
  (|CallParentFunction))

(fn PlaceObstacle
  (bind _spawnedactor (CallFunction|SpawnActor))
  (Transformation|SetActorLocation _spawnedactor (Transformation|GetActorLocation) false false))

(fn SpawnActor
  (bind _spawnedactor (|CallParentFunction))
  (return _spawnedactor))