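; BP_SpawnerPickUp is a spawner that places random pickups at its own location while the level is playing.
; It polls the level manager on a timer until play starts, then runs a self-repeating random-delay loop.
; Each pickup is picked from an actor class array, spawned away from the player, handed a spawner reference and moved into place.
; Actors reported through GetActorHitBounds are destroyed.
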(event Custom|LineUpNextPickUpSpawn
  (Utilities|FlowControl|Delay (Math|Random|RandomFloatinRange (Variables|Default|GetMinDelay) (Variables|Default|GetMaxDelay)))
  (CallFunction|PlacePickUp)
  (if (Variables|/Game/Blueprints/Game/BP_LevelManager.BP_LevelManager_C|GetIsPlaying (Variables|Default|GetLevelManagerRef))
    (CallFunction|LineUpNextPickUpSpawn)))

(event Custom|CheckIfPlaying
  (if (Variables|/Game/Blueprints/Game/BP_LevelManager.BP_LevelManager_C|GetIsPlaying (Variables|Default|GetLevelManagerRef))
    (CallFunction|LineUpNextPickUpSpawn)
    (Utilities|Time|ClearTimerbyFunctionName 0 "CheckIfPlaying")))

(event EventBeginPlay
  (bind (_output _isvalid) (CallFunction|GetLevelManager))
  (if _isvalid
    (Variables|Default|SetLevelManagerRef _output)
    (if (Variables|/Game/Blueprints/Game/BP_LevelManager.BP_LevelManager_C|GetIsPlaying (Variables|Default|GetLevelManagerRef))
      (CallFunction|LineUpNextPickUpSpawn)
      (else
        (Utilities|Time|SetTimerbyEvent (delegate Custom|CheckIfPlaying) 1.0 true)))))

(event EventGetActorHitBounds
  (params (OutOfBoundsActor :type Actor%20Object%20Reference))
  (Actor|DestroyActor OutOfBoundsActor))

(fn ConstructionScript
  (|CallParentFunction))

(fn PlacePickUp
  (bind _spawnedactor (CallFunction|SpawnActor))
  (Transformation|SetActorLocation _spawnedactor (Transformation|GetActorLocation) false false))

(fn SpawnActor
  (bind _actors (Variables|Default|GetActors))
  ;[1 1 1] Spawn away from player
  (bind _returnvalue (Game|SpawnActorfromClass (Utilities|Array|Get(acopy) _actors (Math|Random|RandomIntegerinRange 0 (Utilities|Array|LastIndex _actors))) (Math|Transform|MakeTransform "0.000000, 0,1000.000000" "0, 0, 0" "1,1,1") "Undefined" 0 0))
  (Class|BPISpawnable|SetParent(Message) _returnvalue self)
  (return _returnvalue))