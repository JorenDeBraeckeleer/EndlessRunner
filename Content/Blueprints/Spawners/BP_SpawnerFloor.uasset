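; Floor spawner, a child of a parent spawner, that keeps a row of tiles going along X by recycling them.
; On BeginPlay it spawns NrActors tiles end to end from its own location, taking tile length from the first one's bounds.
; Tiles reported out of bounds move one length beyond RearTile and become the new RearTile.
; A short Delay before that move avoids reading a wrong RearTile location.
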(event EventBeginPlay
  (|CallParentFunction)
  (for _index (range 1 (Variables|Default|GetNrActors))
    (if (== _index 1)
      (bind _spawnedactor (CallFunction|SpawnActor))
      (bind _output_get (Variables|Default|SetRearTile _spawnedactor))
      (Variables|Default|SetTileSize (* (.x (.BoxExtent (Collision|GetActorBounds _output_get false false))) 2.0))
      (Transformation|SetActorLocation (Variables|Default|GetRearTile) (Transformation|GetActorLocation) false false)
      (else
        (bind _spawnedactor_2 (CallFunction|SpawnActor))
        (Transformation|SetActorLocation _spawnedactor_2 (Math|Vector|MakeVector (+ (.x (Transformation|GetActorLocation (Variables|Default|GetRearTile))) (Variables|Default|GetTileSize)) (.y (Transformation|GetActorLocation (Variables|Default|GetRearTile))) (.z (Transformation|GetActorLocation (Variables|Default|GetRearTile)))) false false)
        (Variables|Default|SetRearTile _spawnedactor_2)))))

(event EventGetActorHitBounds
  (params (OutOfBoundsActor :type Actor%20Object%20Reference))
  ;[1 1 1] Without this the wrong location for the RearTile is taken and will not be placed on the correct spot because of this
  (Utilities|FlowControl|Delay 0.01)
  (Transformation|SetActorLocation OutOfBoundsActor (Math|Vector|MakeVector (+ (.x (Transformation|GetActorLocation (Variables|Default|GetRearTile))) (Variables|Default|GetTileSize)) (.y (Transformation|GetActorLocation (Variables|Default|GetRearTile))) (.z (Transformation|GetActorLocation (Variables|Default|GetRearTile)))) false false)
  (Variables|Default|SetRearTile OutOfBoundsActor))

(fn ConstructionScript
  (|CallParentFunction))

(fn SpawnActor
  (bind _spawnedactor (|CallParentFunction))
  (return _spawnedactor))