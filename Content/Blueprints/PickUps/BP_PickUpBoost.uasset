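; BP_PickUpBoost is a pickup that gives a boost to the pawn that touches it.
; Overlap on either of its two static meshes casts the other actor to BP_PawnBase, stores it as Player and calls PickUp.
; The PickUp override calls Boost on that pawn, then runs the parent pickup logic.
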(event OnComponentBeginOverlap(StaticMesh1)
  (params (OverlappedComponent :type Primitive%20Component%20Object%20Reference) (OtherActor :type Actor%20Object%20Reference) (OtherComp :type Primitive%20Component%20Object%20Reference) (OtherBodyIndex :type Integer) (bFromSweep :type Boolean) (SweepResult :type Hit%20Result%20Structure%20%28by%20ref%29))
  (bind _asbp_pawn_base (Utilities|Casting|CastToBP_PawnBase OtherActor))
  (Variables|Default|SetPlayer _asbp_pawn_base)
  (CallFunction|PickUp))

(event OnComponentBeginOverlap(StaticMesh2)
  (params (OverlappedComponent :type Primitive%20Component%20Object%20Reference) (OtherActor :type Actor%20Object%20Reference) (OtherComp :type Primitive%20Component%20Object%20Reference) (OtherBodyIndex :type Integer) (bFromSweep :type Boolean) (SweepResult :type Hit%20Result%20Structure%20%28by%20ref%29))
  (bind _asbp_pawn_base (Utilities|Casting|CastToBP_PawnBase OtherActor))
  (Variables|Default|SetPlayer _asbp_pawn_base)
  (CallFunction|PickUp))

(fn ConstructionScript
  (|CallParentFunction))

(fn PickUp
  (Default|Boost (Variables|Default|GetPlayer))
  (|CallParentFunction))